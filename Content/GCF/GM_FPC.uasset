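; First-person game mode that creates the HUD and respawns the player when their character is destroyed.
; BeginPlay caches the first PlayerStart's transform and binds to the character's OnDestroyed event.
; After a short delay, that event spawns and possesses a new FPC at the cached transform.
; Respawn then resets the HUD key count, fades the camera in and rebinds OnDestroyed to the new character.
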(event `self.ReceiveBeginPlay`
  (`|ExecutionSequence`
    (:`then_0`
      ;[1 1 1] Add HUD to Viewport
      (bind _returnvalue (`|CreateWidget` "/Game/GCF/Widgets/WBP_HUD.WBP_HUD_C"))
      (bind _output_get (set `self.HUD_Ref` _returnvalue))
      (`UserWidget.AddToViewport` _output_get 0))
    (:`then_2`
      ;[1 1 1] Set Spawn from Player Start Actor's Location
      (bind _returnvalue_2 (`GameplayStatics.GetActorOfClass` "/Script/Engine.PlayerStart"))
      (set `self.Spawn Transform` (`self.GetTransform` _returnvalue_2)))
    (:`then_3`
      ;[1 1 1] Respawn
      (add `self.OnDestroyed` (`GameplayStatics.GetPlayerCharacter` 0) (delegate `OnDestroyed_Event_0`) :!label _label))))

(event `Respawn`
  (bind _returnvalue (`GameplayStatics.GetPlayerController` 0))
  ;[1 1 1] Respawn
  (`|ExecutionSequence`
    (:`then_0`
      (bind _foundwidgets (`WidgetBlueprintLibrary.GetAllWidgetsOfClass` "/Game/GCF/Widgets/WBP_HUD.WBP_HUD_C"))
      (for _array_element _foundwidgets
        (`/Game/GCF/Widgets/WBP_HUD.UpdateKeys` _array_element 0)))
    (:`then_1`
      (cast `/Game/GCF/FPC_Controller` _returnvalue)
      (`PlayerCameraManager.StartCameraFade` :`self` (`PlayerController.PlayerCameraManager` _returnvalue) :`FromAlpha` 1.0 :`Duration` 2.0))
    (:`then_2`
      (goto _label))))

(event `OnDestroyed_Event_0` :!signature `self.OnDestroyed`
  (params (DestroyedActor :type "Actor Object Reference"))
  ;[1 1 1] Respawn
  (`|ExecutionSequence`
    (:`then_1`
      (`KismetSystemLibrary.Delay` 2.0)
      (bind _returnvalue (`|SpawnActorFromClass` "/Game/GCF/FPC.FPC_C" (`self.Spawn Transform`) "Undefined" "OverrideRootScale" null null))
      (`Controller.Possess` (`GameplayStatics.GetPlayerController` 0) _returnvalue)
      (`self.Respawn`))))

(fn `UserConstructionScript`)