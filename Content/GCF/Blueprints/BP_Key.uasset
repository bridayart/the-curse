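; BP_Key is a key pickup that adds its KeyValue to the player's key count.
; Any overlap with TGR_Sphere increments KeyCount on the first player's FPC_Controller without checking the overlapping actor, then plays a rattle sound.
; If the game mode is GM_FPC, it loops over top-level WBP_HUD widgets and destroys itself.
; The loop body is empty, as the UpdateKeys HUD call is disconnected.
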(event `self.TGR_Sphere.OnComponentBeginOverlap`
  (params (OverlappedComponent :type "PrimitiveComponent Object Reference") (OtherActor :type "Actor Object Reference") (OtherComp :type "PrimitiveComponent Object Reference") (OtherBodyIndex :type Integer) (bFromSweep :type Boolean) (SweepResult :type "HitResult Structure (by ref)"))
  (bind _asfpc_controller (cast `/Game/GCF/FPC_Controller` (`GameplayStatics.GetPlayerController` 0)))
  (bind _output_get (set `/Game/GCF/FPC_Controller.KeyCount` (+ (`/Game/GCF/FPC_Controller.KeyCount` _asfpc_controller) (`self.KeyValue`)) _asfpc_controller))
  (`GameplayStatics.PlaySoundAtLocation` "/Game/Level1/Audio/KeyRattle_Cue.KeyRattle_Cue" (`self.K2_GetActorLocation`) (struct) 1.0 1.0 0.0 null null null)
  (cast `/Game/GCF/GM_FPC` (`GameplayStatics.GetGameMode`))
  (bind _foundwidgets (`WidgetBlueprintLibrary.GetAllWidgetsOfClass` "/Game/GCF/Widgets/WBP_HUD.WBP_HUD_C"))
  (for _array_element _foundwidgets
    _)
  (`self.K2_DestroyActor`))

(fn `UserConstructionScript`)