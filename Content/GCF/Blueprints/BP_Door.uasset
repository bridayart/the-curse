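; BP_Door is an interactive swinging door that the player opens and closes with the Interact input.
; The TGR_box trigger enables input on overlap and disables it on exit, using player controller 0.
; Interact toggles DoorOpen and plays or reverses a timeline that drives DoorA's relative yaw.
; Opening plays an unlock sound immediately, while closing waits briefly before its sound and reversed swing.
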(event `self.TGR_box.OnComponentBeginOverlap`
  (params (OverlappedComponent :type "PrimitiveComponent Object Reference") (OtherActor :type "Actor Object Reference") (OtherComp :type "PrimitiveComponent Object Reference") (OtherBodyIndex :type Integer) (bFromSweep :type Boolean) (SweepResult :type "HitResult Structure (by ref)"))
  (`self.EnableInput` (`GameplayStatics.GetPlayerController` 0)))

(event `self.TGR_box.OnComponentEndOverlap`
  (params (OverlappedComponent :type "PrimitiveComponent Object Reference") (OtherActor :type "Actor Object Reference") (OtherComp :type "PrimitiveComponent Object Reference") (OtherBodyIndex :type Integer))
  (`self.DisableInput` (`GameplayStatics.GetPlayerController` 0)))

(event `InputAction|Interact`
  (params (Key :type "Key Structure"))
  (bind _returnvalue (`self.K2_GetActorLocation`))
  (:`Pressed`
    (if (`self.DoorOpen?`)
      (set `self.DoorOpen?` false)
      (`KismetSystemLibrary.Delay` 0.2)
      (`GameplayStatics.PlaySoundAtLocation` "/Game/GCF/Audio/DoorClosing_Cue.DoorClosing_Cue" _returnvalue (struct) 1.0 1.0 0.0 null null null)
      (bind (_direction _door_swing) (`Timeline|Timeline_0` :!via `Reverse` :!label _label)
        (:`Update`
          (`SceneComponent.K2_SetRelativeRotation` (`self.Door_a`) (`KismetMathLibrary.MakeRotator` 0.0 0.0 _door_swing) false false)))
      (else
        (set `self.DoorOpen?` true)
        (`GameplayStatics.PlaySoundAtLocation` "/Game/GCF/Audio/UnlockedDoor_Cue.UnlockedDoor_Cue" _returnvalue (struct) 1.0 1.0 0.0 null null null)
        (goto _label)))))

(fn `UserConstructionScript`)