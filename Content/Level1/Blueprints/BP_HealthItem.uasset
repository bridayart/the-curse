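; BP_HealthItem is a health pickup that the player collects by pressing Interact.
; Overlapping its trigger sphere enables input on the actor and shows a WBP_PressE prompt, and ending overlap reverses both.
; Interact routes healing through ApplyDamage on the FPC character using BaseHeal, plays a pill bottle sound at world origin, then destroys the item.
; The overlap events do not check which actor triggered them.
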(event `self.TGR_Sphere.OnComponentBeginOverlap`
  (params (OverlappedComponent :type "PrimitiveComponent Object Reference") (OtherActor :type "Actor Object Reference") (OtherComp :type "PrimitiveComponent Object Reference") (OtherBodyIndex :type Integer) (bFromSweep :type Boolean) (SweepResult :type "HitResult Structure (by ref)"))
  ;[1 1 1] Enable Input
  (`self.EnableInput` (`GameplayStatics.GetPlayerController` 0))
  (bind _returnvalue (`|CreateWidget` "/Game/GCF/Widgets/WBP_PressE.WBP_PressE_C"))
  (bind _output_get (set `self.Press E Ref` _returnvalue))
  (`UserWidget.AddToViewport` _output_get 0))

(event `self.TGR_Sphere.OnComponentEndOverlap`
  (params (OverlappedComponent :type "PrimitiveComponent Object Reference") (OtherActor :type "Actor Object Reference") (OtherComp :type "PrimitiveComponent Object Reference") (OtherBodyIndex :type Integer))
  ;[1 1 1] Enable Input
  (`self.DisableInput` (`GameplayStatics.GetPlayerController` 0))
  (`Widget.RemoveFromParent` (`self.Press E Ref`)))

(event `InputAction|Interact`
  (params (Key :type "Key Structure"))
  (:`Pressed`
    (bind _asfpc (cast `/Game/GCF/FPC` (`GameplayStatics.GetPlayerCharacter` 0)))
    (`GameplayStatics.ApplyDamage` _asfpc (`self.Base Heal`) null self)
    (`GameplayStatics.PlaySoundAtLocation` "/Game/Level1/Audio/PillBottle_Cue.PillBottle_Cue" (0.0 0.0 0.0) (struct) 1.0 1.0 0.0 null null null)
    (`self.K2_DestroyActor`)))

(fn `UserConstructionScript`)