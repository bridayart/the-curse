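; BP_KeyInteract2 is a key pickup in Level1 that the player collects with the Interact input.
; Overlapping its trigger sphere enables actor input and shows a WBP_PressE prompt; leaving reverses both.
; Interacting increments KeyCount on FPC_Controller, plays a key rattle, pushes the count to WBP_HUD and destroys the actor.
; A second sequence branch also plays a laugh sound at the key's location.
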(event `self.TGR_Sphere.OnComponentBeginOverlap`
  (params (OverlappedComponent :type "PrimitiveComponent Object Reference") (OtherActor :type "Actor Object Reference") (OtherComp :type "PrimitiveComponent Object Reference") (OtherBodyIndex :type Integer) (bFromSweep :type Boolean) (SweepResult :type "HitResult Structure (by ref)"))
  ;[1 1 1] Enable Input
  (`self.EnableInput` (`GameplayStatics.GetPlayerController` 0))
  (bind _returnvalue (`|CreateWidget` "/Game/GCF/Widgets/WBP_PressE.WBP_PressE_C"))
  (bind _output_get (set `self.Press E Ref` _returnvalue))
  (`UserWidget.AddToViewport` _output_get 0))

(event `self.TGR_Sphere.OnComponentEndOverlap`
  (params (OverlappedComponent :type "PrimitiveComponent Object Reference") (OtherActor :type "Actor Object Reference") (OtherComp :type "PrimitiveComponent Object Reference") (OtherBodyIndex :type Integer))
  ;[1 1 1] Enable Input
  (`self.DisableInput` (`GameplayStatics.GetPlayerController` 0))
  (`Widget.RemoveFromParent` (`self.Press E Ref`)))

(event `InputAction|Interact`
  (params (Key :type "Key Structure"))
  (:`Pressed`
    (bind _asfpc_controller (cast `/Game/GCF/FPC_Controller` (`GameplayStatics.GetPlayerController` 0)))
    (bind _output_get (set `/Game/GCF/FPC_Controller.KeyCount` (+ (`/Game/GCF/FPC_Controller.KeyCount` _asfpc_controller) 1) _asfpc_controller))
    (`|ExecutionSequence`
      (:`then_0`
        (`GameplayStatics.PlaySoundAtLocation` "/Game/Level1/Audio/KeyRattle_Cue.KeyRattle_Cue" (`self.K2_GetActorLocation`) (struct) 1.0 1.0 0.0 null null null)
        (bind _foundwidgets (`WidgetBlueprintLibrary.GetAllWidgetsOfClass` "/Game/GCF/Widgets/WBP_HUD.WBP_HUD_C"))
        (for _array_element _foundwidgets
          (`/Game/GCF/Widgets/WBP_HUD.UpdateKeys` _array_element _output_get))
        (`self.K2_DestroyActor`))
      (:`then_1`
        (`GameplayStatics.PlaySoundAtLocation` "/Game/Level1/Audio/Hurt_Laugh_2.Hurt_Laugh_2" (`self.K2_GetActorLocation`) (struct) 1.0 1.0 0.0 null null null)))))

(fn `UserConstructionScript`)